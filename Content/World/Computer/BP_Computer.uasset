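; BP_Computer is an interactable computer in the world that shows an on-screen widget when used.
; Interface events drive it: focus shows hover text and an outline overlay material on the cube, and losing focus clears both.
; Interacting shows the computer widget and blends the player's view to the computer actor, while ending interaction hides it and returns the view to the pawn.
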(event EventBeginPlay
  (Rendering|SetVisibility (Variables|Default|GetHoverText) false false)
  (Rendering|SetVisibility (Variables|Default|GetComputerWidget) false false))

(event EventInteract
  ;[0.15 0.15 0.15 0.5] Interface Events
  (Rendering|SetVisibility (Variables|Default|GetHoverText) false false)
  (Rendering|SetVisibility (Variables|Default|GetComputerWidget) true false)
  (Game|Player|SetViewTargetwithBlend (Game|GetPlayerController 0) self 0.5 "VTBlend_Linear" 0.0 false))

(event EventFocus
  ;[0.15 0.15 0.15 0.5] Interface Events
  (Rendering|SetVisibility (Variables|Default|GetHoverText) true false)
  (Rendering|Material|SetOverlayMaterial (Variables|Default|GetCube) "/Game/FirstPerson/Blueprints/Interaction/M_Outline_Inst.M_Outline_Inst" :!class /Script/Engine.MeshComponent))

(event EventEndFocus
  ;[0.15 0.15 0.15 0.5] Interface Events
  (Rendering|SetVisibility (Variables|Default|GetHoverText) false false)
  (Rendering|Material|SetOverlayMaterial (Variables|Default|GetCube) 0 :!class /Script/Engine.MeshComponent))

(event EventEndInteract
  ;[0.15 0.15 0.15 0.5] Interface Events
  (Rendering|SetVisibility (Variables|Default|GetComputerWidget) false false)
  (Game|Player|SetViewTargetwithBlend (Game|GetPlayerController 0) (Game|Player|GetPlayerPawn 0) 0.0 "VTBlend_Linear" 0.0 false))

(fn ConstructionScript)

(fn GetInteractableType
  (return (Variables|Default|GetInteractableType)))