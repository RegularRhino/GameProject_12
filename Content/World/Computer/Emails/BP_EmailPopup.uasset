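; BP_EmailPopup is a world actor that lets the player open an email popup at a computer.
; Overlapping its MessageCollider reveals a text prompt and enables interaction; leaving hides the prompt and closes any open popup.
; Interact toggles an EmailPopup widget fed with the actor's Emails, switching input mode and mouse cursor to match.
; The widget's close-click dispatcher routes back into Interact to dismiss it.
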(event OnComponentBeginOverlap(MessageCollider)
  (params (OverlappedComponent :type Primitive%20Component%20Object%20Reference) (OtherActor :type Actor%20Object%20Reference) (OtherComp :type Primitive%20Component%20Object%20Reference) (OtherBodyIndex :type Integer) (bFromSweep :type Boolean) (SweepResult :type Hit%20Result%20Structure%20%28by%20ref%29))
  (Rendering|SetVisibility (Variables|Default|GetTextRender) true false)
  (Variables|Default|SetInteractable true))

(event OnComponentEndOverlap(MessageCollider)
  (params (OverlappedComponent :type Primitive%20Component%20Object%20Reference) (OtherActor :type Actor%20Object%20Reference) (OtherComp :type Primitive%20Component%20Object%20Reference) (OtherBodyIndex :type Integer))
  (bind _returnvalue (Game|GetPlayerController 0))
  (Rendering|SetVisibility (Variables|Default|GetTextRender) false false)
  (Variables|Default|SetInteractable false)
  (if (not (== (Variables|Default|GetWidget) 0))
    (Widget|RemovefromParent (Variables|Default|GetWidget))
    (Variables|Default|SetWidget 0)
    (Input|SetInputModeGameOnly _returnvalue false)
    (Variables|/Script/Engine.PlayerController|SetbShowMouseCursor _returnvalue false)))

(event Custom|ED_CloseClicked_Event_0
  (CallFunction|Interact))

(event EventInteract
  (bind _returnvalue (Game|GetPlayerController 0))
  (bind _returnvalue_2 (Game|GetPlayerController 0))
  (if (== (Variables|Default|GetWidget) 0) ; Do we have nothing on the screen
    (if (Variables|Default|GetInteractable) ; Can we interact
      (bind _returnvalue_3 (UserInterface|CreateWidget "/Game/World/Computer/Emails/EmailPopup.EmailPopup_C" (Game|GetPlayerController 0) (Variables|Default|GetEmails)))
      (bind _output_get (Variables|Default|SetWidget _returnvalue_3))
      (UserInterface|Viewport|AddtoViewport _output_get 0)
      (Input|SetInputModeUIOnly _returnvalue 0 "DoNotLock" false)
      (Variables|/Script/Engine.PlayerController|SetbShowMouseCursor _returnvalue true)
      (EventDispatchers|AssignEDCloseClicked (Variables|Default|GetWidget) (delegate Custom|ED_CloseClicked_Event_0)))
    (else
      (Widget|RemovefromParent (Variables|Default|GetWidget))
      (Variables|Default|SetWidget 0)
      (Input|SetInputModeGameOnly _returnvalue_2 false)
      (Variables|/Script/Engine.PlayerController|SetbShowMouseCursor _returnvalue_2 false))))

(event EventBeginPlay
  (Rendering|SetVisibility (Variables|Default|GetTextRender) false false))

(fn ConstructionScript)