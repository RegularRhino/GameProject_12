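; BP_InspectItem is an interactable world item, apparently meant for close inspection by the player.
; On Interact it disables the instigator's input and enables its own for player controller 0; EndInteract is empty, so nothing restores input.
; Mouse-button drag rotation of ItemMesh while IsHeld is present but disconnected, with zeroed axis values.
; It reports its InteractionType, while both folder and file opened queries always return false.
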(event EventInteract
  (params (InteractInstigator :type Actor%20Object%20Reference))
  (bind _returnvalue (Game|GetPlayerController 0))
  (Input|DisableInput InteractInstigator _returnvalue)
  (Input|EnableInput _returnvalue))

(event EventEndInteract)

(fn ConstructionScript)

(fn InteractableType
  (return (Variables|Default|GetInteractionType)))

(fn WasImportantFolderOpened?
  (return false))

(fn WasWizardFileOpened?
  (return false))