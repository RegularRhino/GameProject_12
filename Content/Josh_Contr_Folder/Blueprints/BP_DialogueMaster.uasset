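; NPC dialogue actor that fills a dialogue widget when something overlaps its box.
; Overlap creates WBP_Dialogue, then SetupDialogue uses the NPC enum as a DT_DialogueData row name to set mesh, sound, name and text.
; DialogueIncrease then advances through a separate DialogueLines array, and a timer starts with no function name or AddToViewport call shown.
; End overlap, or running past the last line, pauses the timer and removes the widget.
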(event OnComponentBeginOverlap(Box)
  (params (OverlappedComponent :type Primitive%20Component%20Object%20Reference) (OtherActor :type Actor%20Object%20Reference) (OtherComp :type Primitive%20Component%20Object%20Reference) (OtherBodyIndex :type Integer) (bFromSweep :type Boolean) (SweepResult :type Hit%20Result%20Structure%20%28by%20ref%29))
  (bind _returnvalue (UserInterface|CreateWidget "/Game/Josh_Contr_Folder/UI/Widget_BluePrint/WBP_Dialogue.WBP_Dialogue_C"))
  (Variables|Default|SetDialogueUI _returnvalue)
  (CallFunction|SetupDialogue)
  (CallFunction|DialogueIncrease)
  (bind _returnvalue_2 (Utilities|Time|SetTimerbyFunctionName 0 "" 2.0))
  (Variables|Default|SetDialogueTimer _returnvalue_2))

(event OnComponentEndOverlap(Box)
  (params (OverlappedComponent :type Primitive%20Component%20Object%20Reference) (OtherActor :type Actor%20Object%20Reference) (OtherComp :type Primitive%20Component%20Object%20Reference) (OtherBodyIndex :type Integer))
  (Widget|RemovefromParent (Variables|Default|GetDialogueUI))
  (Utilities|Time|PauseTimerbyHandle (Variables|Default|GetDialogueTimer)))

(event EventBeginPlay
  (AddComponent|AddStaticMeshComponent false (Variables|Default|GetTetoTransform)))

(fn ConstructionScript)

(fn SetupDialogue
  (bind _returnvalue (Utilities|GetDataTableRow "/Game/Josh_Contr_Folder/DataTable/DT_DialogueData.DT_DialogueData" (Utilities|String|StringToName (Utilities|String|EnumtoString (Variables|Default|GetNPCToShow))))
    (:then
      (Development|PrintString "Row Found!")
      (Components|StaticMesh|SetStaticMesh (Variables|Default|GetStaticMesh) (.NPCVisual (Utilities|Struct|BreakStructure_Data _returnvalue)))
      (Variables|Default|SetInteract%20Sound (.InteractSound (Utilities|Struct|BreakStructure_Data _returnvalue)))
      (Rendering|Components|TextRender|SetText (Variables|/Game/Josh_Contr_Folder/UI/Widget_BluePrint/WBP_Dialogue.WBP_Dialogue_C|GetNPC_Name (Variables|Default|GetDialogueUI)) (Utilities|Text|ToText(String) (.NPCName (Utilities|Struct|BreakStructure_Data _returnvalue))))
      (Rendering|Components|TextRender|SetText (Variables|/Game/Josh_Contr_Folder/UI/Widget_BluePrint/WBP_Dialogue.WBP_Dialogue_C|GetNPC_Text (Variables|Default|GetDialogueUI)) (Utilities|Text|ToText(String) (.Dialogue (Utilities|Struct|BreakStructure_Data _returnvalue)))))))

(fn DialogueIncrease
  (Math|Integer|IncrementInt (Variables|Default|GetLineIndex)
    (:%20%20
      (if (<= (Variables|Default|GetLineIndex) (Utilities|Array|Length (Variables|Default|GetDialogueLines)))
        (Rendering|Components|TextRender|SetText (Variables|/Game/Josh_Contr_Folder/UI/Widget_BluePrint/WBP_Dialogue.WBP_Dialogue_C|GetNPC_Text (Variables|Default|GetDialogueUI)) (Utilities|Array|Get(acopy) (Variables|Default|GetDialogueLines) (Variables|Default|GetLineIndex)))
        (else
          (Utilities|Time|PauseTimerbyHandle (Variables|Default|GetDialogueTimer))
          (Widget|RemovefromParent (Variables|Default|GetDialogueUI)))))))