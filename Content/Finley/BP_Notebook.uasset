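; BP_Notebook is an interactable notebook that shows instruction text in a close-up view while the player interacts with it.
; Interact reveals InstructionText and blends the player's view target to the notebook actor, while EndInteract hides it and blends back to the pawn.
; It reports a fixed interactable type, and its folder and wizard-file queries always return false.
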(event EventBeginPlay
  (Rendering|SetVisibility (Variables|Default|GetInstructionText) false false))

(event EventInteract
  (params (InteractInstigator :type Actor%20Object%20Reference))
  (Rendering|SetVisibility (Variables|Default|GetInstructionText) true false)
  (Game|Player|SetViewTargetwithBlend (Game|GetPlayerController 0) self 0.5 "VTBlend_Linear" 0.0 false))

(event EventEndInteract
  (params (DialogueFinalChoice :type Integer))
  (Rendering|SetVisibility (Variables|Default|GetInstructionText) false false)
  (Game|Player|SetViewTargetwithBlend (Game|GetPlayerController 0) (Game|Player|GetPlayerPawn 0) 0.5 "VTBlend_Linear" 0.0 false))

(fn ConstructionScript)

(fn InteractableType
  (return "NewEnumerator4"))

(fn WasImportantFolderOpened?
  (return false))

(fn WasWizardFileOpened?
  (return false))