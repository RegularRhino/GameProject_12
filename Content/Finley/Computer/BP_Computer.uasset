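; Interactable computer actor that shows a screen widget and tracks whether its task is complete and the wizard file was opened.
; Interface events show or hide the screen, blend the camera between computer and player pawn, and toggle typing sounds.
; SetDayCount initializes the screen with a zero-based day index.
; Screen dispatchers bound on BeginPlay set the two progress flags, which getter functions expose.
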(event Custom|HandleFileUnlocked
  ;[0.3916 0.02315 0.03955 0.502] Sets the visibilty of the screen and binds event dispatchers with a cast
  (Variables|Default|SetTaskComplete? true))

(event Custom|HandleWizardFileUnlocked
  ;[0.3916 0.02315 0.03955 0.502] Sets the visibilty of the screen and binds event dispatchers with a cast
  (Variables|Default|SetWizardFileOpened true))

(event EventBeginPlay
  (bind _computerwidget (Variables|Default|GetComputerWidget))
  ;[0.3916 0.02315 0.03955 0.502] Sets the visibilty of the screen and binds event dispatchers with a cast
  (Rendering|SetVisibility _computerwidget false false)
  (bind _aswbp_screen (Utilities|Casting|CastToWBP_Screen (UserInterface|GetWidget _computerwidget)))
  (Variables|Default|SetScreenRef _aswbp_screen)
  (EventDispatchers|BindEventtoTaskComplete (Variables|Default|GetScreenRef) (delegate Custom|HandleFileUnlocked))
  (EventDispatchers|BindEventtoUnlockedWizardFile (Variables|Default|GetScreenRef) (delegate Custom|HandleWizardFileUnlocked))
  (Components|Activation|SetActive (Variables|Default|GetTypingSounds) false false))

(event EventSetDayCount
  (params (DayCount :type Integer))
  ;[0.3906 0.02319 0.03928 0.5] Interface Events
  (Default|Initialize (Variables|Default|GetScreenRef) (- DayCount 1)))

(event EventFocus
  ;[0.3906 0.02319 0.03928 0.5] Interface Events
)

(event EventEndFocus
  ;[0.3906 0.02319 0.03928 0.5] Interface Events
)

(event EventEndInteract
  (Rendering|SetVisibility (Variables|Default|GetComputerWidget) false false)
  (Game|Player|SetViewTargetwithBlend (Game|GetPlayerController 0) (Game|Player|GetPlayerPawn 0) 0.5 "VTBlend_Linear" 0.0 false)
  (Components|Activation|SetActive (Variables|Default|GetTypingSounds) false false))

(event EventInteract
  (params (InteractInstigator :type Actor%20Object%20Reference))
  (Audio|PlaySound2D "/Game/SoundEffects/SW_ComputerStartup.SW_ComputerStartup" 0.75 1.0 0.0 0 0)
  (Rendering|SetVisibility (Variables|Default|GetComputerWidget) true false)
  (Game|Player|SetViewTargetwithBlend (Game|GetPlayerController 0) self 0.5 "VTBlend_Linear" 0.0 false)
  (Components|Activation|SetActive (Variables|Default|GetTypingSounds) true false))

(fn ConstructionScript)

(fn GetInteractableType
  (return "NewEnumerator0"))

(fn WasTaskComplete?
  (return (Variables|Default|GetTaskComplete?)))

(fn WasWizardFileOpened?
  (return (Variables|Default|GetWizardFileOpened)))