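; BP_TempLamp is an interactable lamp whose main light can be switched off and on.
; The Construction Script applies configurable intensities to the main and ambient lights.
; Interact uses a FlipFlop to alternate MainLight between zero and its configured intensity, starting with off, while AmbientLight stays unchanged.
; Focus and EndFocus toggle custom depth rendering on the static mesh.
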(event EventBeginPlay)

(event Collision|EventActorBeginOverlap
  (params (OtherActor :type Actor%20Object%20Reference)))

(event EventTick
  (params (DeltaSeconds :type Float%20%28single-precision%29)))

(event EventInteract
  (Utilities|FlowControl|FlipFlop
    (:A
      (Rendering|Components|Light|SetIntensity (Variables|Default|GetMainLight) 0.0))
    (:B
      (Rendering|Components|Light|SetIntensity (Variables|Default|GetMainLight) (Variables|Default|GetMainLightIntensity)))))

(event EventFocus
  (Rendering|SetRenderCustomDepth (Variables|Default|GetStaticMesh) true))

(event EventEndFocus
  (Rendering|SetRenderCustomDepth (Variables|Default|GetStaticMesh) false))

(fn ConstructionScript
  (Rendering|Components|Light|SetIntensity (Variables|Default|GetMainLight) (Variables|Default|GetMainLightIntensity))
  (Rendering|Components|Light|SetIntensity (Variables|Default|GetAmbientLight) (Variables|Default|GetAmbientLightIntensity)))