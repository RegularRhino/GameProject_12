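; Player interaction component that lets the player focus and use world actors implementing BPI_InteractionInterface.
; A looping timer line-traces from the camera, sending focus messages and filling the crosshair material when it finds an interactable.
; IA_Interact messages the target; Important types also hide the crosshair, show the cursor and pause tracing until IA_EndInteract restores gameplay.
; An intro cutscene snippet is left unconnected.
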(event Custom|TraceForInteractable
  (if (not (Variables|Default|GetIsInteracting))
    (bind (_hitactor _didhit) (CallFunction|InteractionTrace))
    (if _didhit
      (if (Utilities|DoesObjectImplementInterface _hitactor "/Game/Finley/Player/BPI_InteractionInterface.BPI_InteractionInterface_C")
        (CallFunction|FoundInteractable _hitactor)
        (else
          (CallFunction|NoInteractableFound :!label _label)))
      (else
        (goto _label)))))

(event Custom|Setup)

(event Input|EnhancedActionEvents|EnhancedInputActionIA_EndInteract
  (params (ActionValue :type Boolean) (ElapsedSeconds :type Float%20%28double-precision%29) (TriggeredSeconds :type Float%20%28double-precision%29) (InputAction :type Input%20Action%20Object%20Reference :default "/Game/Input/Actions/IA_EndInteract.IA_EndInteract"))
  (bind _returnvalue (Game|GetPlayerController 0))
  (:Started
    (if (Variables|Default|GetIsInteracting)
      (Utilities|IsValid (Variables|Default|GetTargetInteractable)
        (:Is%20Valid
          (Input|SetInputModeGameOnly _returnvalue false)
          (Variables|/Script/Engine.PlayerController|SetbShowMouseCursor _returnvalue false)
          (Class|BPIInteractionInterface|EndInteract(Message) (Variables|Default|GetTargetInteractable))
          (Variables|Default|SetIsInteracting false)
          (Widget|SetVisibility (Variables|Default|GetCrosshairRef) "Visible"))))))

(event Input|EnhancedActionEvents|EnhancedInputActionIA_Interact
  (params (ActionValue :type Boolean) (ElapsedSeconds :type Float%20%28double-precision%29) (TriggeredSeconds :type Float%20%28double-precision%29) (InputAction :type Input%20Action%20Object%20Reference :default "/Game/Input/Actions/IA_Interact.IA_Interact"))
  (bind _returnvalue (Game|GetPlayerController 0))
  (bind _targetinteractable (Variables|Default|GetTargetInteractable))
  (:Started
    (Utilities|IsValid _targetinteractable
      (:Is%20Valid
        (bind _interactabletype (Class|BPIInteractionInterface|GetInteractableType(Message) _targetinteractable))
        (switch Utilities|FlowControl|Switch|SwitchonE_InteractableType _interactabletype
          (:NewEnumerator0
            (Widget|SetVisibility (Variables|Default|GetCrosshairRef) "Collapsed")
            (Input|SetInputModeGameandUI _returnvalue 0 "DoNotLock" true false)
            (Variables|/Script/Engine.PlayerController|SetbShowMouseCursor _returnvalue true)
            (Class|BPIInteractionInterface|Interact(Message) (Variables|Default|GetTargetInteractable))
            (Variables|Default|SetIsInteracting true))
          (:NewEnumerator2
            (Class|BPIInteractionInterface|Interact(Message) (Variables|Default|GetTargetInteractable))))))))

(event EventBeginPlay
  (Variables|Default|SetPlayerRef (Components|GetOwner))
  (Input|SetIgnoreMoveInput (Game|GetPlayerController 0) false)
  (bind _returnvalue (UserInterface|CreateWidget "/Game/Finley/WBP_Crosshair.WBP_Crosshair_C"))
  (bind _output_get (Variables|Default|SetCrosshairRef _returnvalue))
  (UserInterface|Viewport|AddtoViewport _output_get 0)
  (Utilities|Time|SetTimerbyEvent (delegate Custom|TraceForInteractable) 0.2 true))

(fn InteractionTrace
  (bind _returnvalue (Game|GetPlayerCameraManager 0))
  (bind _returnvalue_2 (Transformation|GetActorLocation _returnvalue))
  (bind (_outhit _returnvalue_3) (Collision|LineTraceByChannel _returnvalue_2 (+ _returnvalue_2 (* (Transformation|GetActorForwardVector _returnvalue) (LocalVariables|GetInteractionDistance))) "TraceTypeQuery3" false 0 "None"))
  (return (.HitActor (Collision|BreakHitResult _outhit)) _returnvalue_3))

(fn FoundInteractable
  (params (TargetInteractable :type Actor%20Object%20Reference))
  (bind _output_get (Variables|Default|SetTargetInteractable TargetInteractable))
  (bind _returnvalue (Appearance|GetDynamicMaterial (Variables|/Game/Finley/WBP_Crosshair.WBP_Crosshair_C|GetCrosshair (Variables|Default|GetCrosshairRef)) :!class /Script/UMG.Image))
  (Rendering|Material|SetScalarParameterValue _returnvalue "FillOpacity" 1.0 :!class /Script/Engine.MaterialInstanceDynamic)
  (Class|BPIInteractionInterface|Focus(Message) _output_get))

(fn NoInteractableFound
  (Class|BPIInteractionInterface|EndFocus(Message) (Variables|Default|GetTargetInteractable))
  (Variables|Default|SetTargetInteractable 0)
  (bind _returnvalue (Appearance|GetDynamicMaterial (Variables|/Game/Finley/WBP_Crosshair.WBP_Crosshair_C|GetCrosshair (Variables|Default|GetCrosshairRef)) :!class /Script/UMG.Image))
  (Rendering|Material|SetScalarParameterValue _returnvalue "FillOpacity" 0.0 :!class /Script/Engine.MaterialInstanceDynamic))